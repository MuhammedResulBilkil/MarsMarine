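; BP_MissionAreaVolume is a mission boundary volume that punishes the player for leaving the mission area.
; When a BP_Marine stops overlapping it, the volume sets that marine's OutsideMissionArea flag and starts a five-second KillPlayer timer.
; Re-entering clears both the flag and the timer.
; If the timer expires, KillPlayer applies heavy damage to player character 0, regardless of which marine left.
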(event `self.ReceiveActorBeginOverlap`
  (params (OtherActor :type "Actor Object Reference"))
  (bind _asbp_marine (cast `/Game/Blueprints/Pawns/BP_Marine` OtherActor))
  (`/Engine/EditorBlueprintResources/StandardMacros.IsValid` _asbp_marine
    (:`Is Valid`
      (set `/Game/Blueprints/Pawns/BP_Marine.OutsideMissionArea` false _asbp_marine)
      (`KismetSystemLibrary.K2_ClearTimer` null "KillPlayer"))))

(event `self.ReceiveActorEndOverlap`
  (params (OtherActor :type "Actor Object Reference"))
  (bind _asbp_marine (cast `/Game/Blueprints/Pawns/BP_Marine` OtherActor))
  (`/Engine/EditorBlueprintResources/StandardMacros.IsValid` _asbp_marine
    (:`Is Valid`
      (set `/Game/Blueprints/Pawns/BP_Marine.OutsideMissionArea` true _asbp_marine)
      (`KismetSystemLibrary.K2_SetTimer` null "KillPlayer" 5.0))))

(fn `KillPlayer`
  (`GameplayStatics.ApplyDamage` (`GameplayStatics.GetPlayerCharacter` 0) 100.0))

(fn `UserConstructionScript`)