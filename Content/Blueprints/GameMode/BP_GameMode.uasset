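; Game mode that runs endless, escalating waves of alien enemies, starting shortly after play begins.
; Each wave multiplies the rounded difficulty to set its alien count, then a looping timer spawns BP_Alien at random TargetPoints until the count runs out.
; Spawned aliens are tracked in an array; when RemoveAlien empties it with no spawns remaining, the next wave starts after a short delay.
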(event `self.ReceiveBeginPlay`
  (`KismetSystemLibrary.Delay` 2.0)
  (`self.StartNewWave`))

(event `SpawnWave`
  (`self.SpawnAlien`))

(event `EndWave`
  (`KismetSystemLibrary.Delay` 2.0)
  (`self.StartNewWave`))

(fn `GetRandomSpawnPoint`
  (returns (RandomSpawnPoint :type "TargetPoint Object Reference"))
  (bind _outactors (`GameplayStatics.GetAllActorsOfClass` "/Script/Engine.TargetPoint"))
  (return (`|GetArrayItem` _outactors (`KismetMathLibrary.RandomIntegerInRange` 0 (`KismetArrayLibrary.Array_LastIndex` _outactors)))))

(fn `IncreaseWaveDifficulty`
  (bind _output_get (set `self.WaveDifficulty` (`KismetMathLibrary.Round` (* (`self.WaveDifficulty`) (`self.WaveMultiplier`)))))
  (set `self.AlienSpawnsRemaining` _output_get))

(fn `IsWaveComplete`
  (returns (ReturnValue :type Boolean))
  (return (and (== (`KismetArrayLibrary.Array_Length` (`self.Aliens`)) 0) (<= (`self.AlienSpawnsRemaining`) 0))))

(fn `RemoveAlien`
  (params (`Alien To Remove` :type "/Game/Blueprints/AI/BP_Alien Object Reference (by ref)"))
  (`KismetArrayLibrary.Array_RemoveItem` (`self.Aliens`) `Alien To Remove`)
  (if (`self.IsWaveComplete`)
    (`self.EndWave`)))

(fn `SpawnAlien`
  (bind _randomspawnpoint (`self.GetRandomSpawnPoint`))
  (`/Engine/EditorBlueprintResources/StandardMacros.IsValid` _randomspawnpoint
    (:`Is Valid`
      (bind _returnvalue (`|SpawnActorFromClass` "/Game/Blueprints/AI/BP_Alien.BP_Alien_C" (`self.GetTransform` _randomspawnpoint) "Undefined" "OverrideRootScale" null null))
      (`/Engine/EditorBlueprintResources/StandardMacros.IsValid` _returnvalue
        (:`Is Valid`
          (`KismetArrayLibrary.Array_Add` (`self.Aliens`) _returnvalue)
          (bind _result (`/Engine/EditorBlueprintResources/StandardMacros.DecrementInt` (`self.AlienSpawnsRemaining`))
            (:`  `
              (if (<= _result 0)
                (`KismetSystemLibrary.K2_ClearTimer` null "SpawnWave")))))))))

(fn `StartNewWave`
  (`/Engine/EditorBlueprintResources/StandardMacros.IncrementInt` (`self.CurrentWave`)
    (:`  `
      (`self.IncreaseWaveDifficulty`)
      (`KismetSystemLibrary.K2_SetTimer` null "SpawnWave" (`self.AlienSpawnFrequency`) true))))

(fn `UserConstructionScript`)