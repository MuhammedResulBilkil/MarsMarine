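; Alien enemy that chases the player, attacks in melee and dies from damage.
; BeginPlay loops AI MoveTo toward the player until death, while Tick checks range and plays the attack montage with movement deactivated until it completes.
; DamagePlayer applies damage to BP_Marine but is not called within this Blueprint.
; AnyDamage lowers health; at zero it stops movement, disables collision, credits the marine's kill and destroys the actor after a delay.
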(event `self.ReceiveAnyDamage`
  (params (Damage :type "Float (single-precision)") (DamageType :type "DamageType Object Reference") (InstigatedBy :type "Controller Object Reference") (DamageCauser :type "Actor Object Reference"))
  (if (not (`self.IsAlienDead`))
    (bind _healthafterdamage (`self.DecreaseHealth` Damage))
    (if (<= _healthafterdamage 0.0)
      (`self.KillAI`)
      (`KismetSystemLibrary.Delay` 3.0)
      (`self.K2_DestroyActor`))))

(event `self.ReceiveBeginPlay`
  (`|AIMoveTo` self (0.0 0.0 0.0) (`GameplayStatics.GetPlayerCharacter` 0) :!label _label
    (:`OnSuccess`
      _)
    (:`OnFail`
      _))
  (`KismetSystemLibrary.Delay` 0.2)
  (if (not (`self.IsAlienDead`))
    (goto _label)))

(event `self.ReceiveTick`
  (params (DeltaSeconds :type "Float (single-precision)"))
  (if (`self.CanAlienAttack`)
    (`ActorComponent.Deactivate` (`self.CharacterMovement`))
    (`|PlayMontage` (`self.Mesh`) "/Game/Characters/Enemy_Great_Spider/Animations/AlienAttackMontage_1.AlienAttackMontage_1"
      (:`OnCompleted`
        (`ActorComponent.Activate` (`self.CharacterMovement`) false)))))

(fn `CanAlienAttack`
  (returns (ReturnValue :type Boolean))
  (return (and (`self.IsInAttackRange`) (not (`self.IsAttacking`)) (not (`self.IsAlienDead`)))))

(fn `DamagePlayer`
  (if (not (`self.IsAlienDead`))
    (bind _asbp_marine (cast `/Game/Blueprints/Pawns/BP_Marine` (`GameplayStatics.GetPlayerPawn` 0)))
    (`GameplayStatics.ApplyDamage` _asbp_marine (`self.DamageAmount`))))

(fn `DeactivateAIMovement`
  (bind _charactermovement (`self.CharacterMovement`))
  (`MovementComponent.StopMovementImmediately` _charactermovement)
  (`ActorComponent.Deactivate` _charactermovement))

(fn `DecreaseHealth`
  (params (DamageAmount :type "Float (double-precision)"))
  (returns (HealthAfterDamage :type "Float (double-precision)"))
  (bind _output_get (set `self.AlienHealth` (- (`self.AlienHealth`) DamageAmount)))
  (return _output_get))

(fn `IsAttacking`
  (returns (ReturnValue :type Boolean))
  (return (`AnimInstance.Montage_IsPlaying` (`SkeletalMeshComponent.GetAnimInstance` (`self.Mesh`)) "/Game/Characters/Enemy_Great_Spider/Animations/AlienAttackMontage_1.AlienAttackMontage_1")))

(fn `IsInAttackRange`
  (returns (ReturnValue :type Boolean))
  (return (<= (`self.GetDistanceTo` (`GameplayStatics.GetPlayerCharacter` 0)) (`self.AttackRange`))))

(fn `KillAI`
  (set `self.IsAlienDead` true)
  (`self.DeactivateAIMovement`)
  (`self.SetActorEnableCollision` false)
  (bind _asbp_marine (cast `/Game/Blueprints/Pawns/BP_Marine` (`GameplayStatics.GetPlayerCharacter` 0)))
  (`/Game/Blueprints/Pawns/BP_Marine.IncreaseKills` _asbp_marine))

(fn `UserConstructionScript`)